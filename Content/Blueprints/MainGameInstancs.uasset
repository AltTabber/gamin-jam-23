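; Game instance Blueprint that manages the game's main menu, pause menu and message screens, and starts new games.
; Show events lazily create and cache each widget, add it to the viewport and switch to UI-only input with a visible cursor.
; The pause and message screens also pause the game; their close events remove the widget, unpause and restore game input.
; CreateNewGame sets game-only input and opens BaseMap.
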(event Custom|ShowMainMenu
  (bind _returnvalue (Game|GetPlayerController 0))
  (Utilities|IsValid (Variables|Widgets|GetMainMenu_WB)
    (:Is%20Valid
      _)
    (:Is%20Not%20Valid
      (bind _returnvalue_2 (UserInterface|CreateWidget "/Game/UI/Menu/MainMenu_BP.MainMenu_BP_C" _returnvalue))
      (Variables|Widgets|SetMainMenu_WB _returnvalue_2)))
  (UserInterface|Viewport|AddtoViewport (Variables|Widgets|GetMainMenu_WB) 0)
  (Variables|/Script/Engine.PlayerController|SetbShowMouseCursor _returnvalue true)
  (Input|SetInputModeUIOnly _returnvalue (Variables|Widgets|GetMainMenu_WB) "LockInFullscreen"))

(event Custom|CreateNewGame
  (Input|SetInputModeGameOnly (Game|GetPlayerController 0))
  (Game|OpenLevel(byName) "BaseMap"))

(event Custom|ShowPauseMenu
  (bind _returnvalue (Game|GetPlayerController 0))
  (Utilities|IsValid (Variables|Widgets|GetPauseMenu_WB)
    (:Is%20Valid
      _)
    (:Is%20Not%20Valid
      (bind _returnvalue_2 (UserInterface|CreateWidget "/Game/UI/Menu/PauseMenu_BP.PauseMenu_BP_C" _returnvalue))
      (Variables|Widgets|SetPauseMenu_WB _returnvalue_2)))
  (UserInterface|Viewport|AddtoViewport (Variables|Widgets|GetPauseMenu_WB) 0)
  (Input|SetInputModeUIOnly _returnvalue (Variables|Widgets|GetPauseMenu_WB) "LockInFullscreen")
  (Game|SetGamePaused true)
  (Variables|/Script/Engine.PlayerController|SetbShowMouseCursor _returnvalue true))

(event Custom|PauseMenuResume
  (bind _returnvalue (Game|GetPlayerController 0))
  (Widget|RemovefromParent (Variables|Widgets|GetPauseMenu_WB))
  (Game|SetGamePaused false)
  (Input|SetInputModeGameOnly _returnvalue)
  (Variables|/Script/Engine.PlayerController|SetbShowMouseCursor _returnvalue false))

(event Custom|ShowMassage
  (bind _returnvalue (Game|GetPlayerController 0))
  (Utilities|IsValid (Variables|Widgets|GetMassage_WB)
    (:Is%20Valid
      _)
    (:Is%20Not%20Valid
      (bind _returnvalue_2 (UserInterface|CreateWidget "/Game/UI/Massage_BP.Massage_BP_C" _returnvalue))
      (Variables|Widgets|SetMassage_WB _returnvalue_2)))
  (UserInterface|Viewport|AddtoViewport (Variables|Widgets|GetMassage_WB) 0)
  (Input|SetInputModeUIOnly _returnvalue (Variables|Widgets|GetMassage_WB) "LockInFullscreen")
  (Game|SetGamePaused true)
  (Variables|/Script/Engine.PlayerController|SetbShowMouseCursor _returnvalue true))

(event Custom|HideMassage
  (bind _returnvalue (Game|GetPlayerController 0))
  (Widget|RemovefromParent (Variables|Widgets|GetMassage_WB))
  (Game|SetGamePaused false)
  (Input|SetInputModeGameOnly _returnvalue)
  (Variables|/Script/Engine.PlayerController|SetbShowMouseCursor _returnvalue false))